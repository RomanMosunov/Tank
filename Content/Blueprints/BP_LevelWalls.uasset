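; BP_LevelWalls is an actor that builds a grid-based wall layout from static mesh components in its Construction Script.
; Nested loops over CountX and CountY place meshes at Spacing intervals, using FilterIndex to always fill the outer border.
; Interior cells get a mesh with a 25% chance from an unseeded random roll, so the layout changes whenever construction reruns.
; The event graph holds no active logic.
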(fn `FilterIndex`
  (returns (Out :type Boolean))
  (bind _indexx (`self.IndexX`))
  (bind _indexy (`self.IndexY`))
  (return (or (== 0 _indexx) (== _indexx (`self.CountX`)) (== 0 _indexy) (== _indexy (`self.CountY`)))))

(fn `UserConstructionScript`
  (bind _returnvalue (* (`self.IndexY`) (`self.Spacing`)))
  (bind _returnvalue_2 (* (`self.IndexX`) (`self.Spacing`)))
  (for _index (range (+ (`self.CountY`) 1))
    (set `self.IndexY` _index)
    (for _index_2 (range (+ (`self.CountX`) 1))
      (set `self.IndexX` _index_2)
      (if (`self.FilterIndex`)
        (`AddComponent|NODE_AddStaticMeshComponent-0` :`RelativeTransform` (`KismetMathLibrary.MakeTransform` (`KismetMathLibrary.MakeVector` _returnvalue_2 _returnvalue)))
        (elif (`KismetMathLibrary.RandomBoolWithWeight` 0.25)
          (`AddComponent|NODE_AddStaticMeshComponent-1` :`RelativeTransform` (`KismetMathLibrary.MakeTransform` (`KismetMathLibrary.MakeVector` _returnvalue_2 _returnvalue))))))))